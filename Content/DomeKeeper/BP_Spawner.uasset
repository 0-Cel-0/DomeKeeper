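; BP_Spawner builds the block field for the DomeKeeper game and owns its score HUD.
; On BeginPlay it spawns a Length by Height grid of BP_BlockCube from its own location, stepping along Y and dropping in Z after each row, with block HP rising per row.
; It then adds a WBP_Score widget to the viewport, and its IncrementScore event tells that widget to add 100 points.
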(event `self.ReceiveBeginPlay`
  (`|ExecutionSequence`
    (:`then_0`
      (`self.Create Blocks`))
    (:`then_1`
      (`self.Create HUD`))))

(event `Create Blocks`
  (bind (_returnvalue_x _returnvalue_y _returnvalue_z) (`KismetMathLibrary.BreakVector` (`self.K2_GetActorLocation`)))
  (set `self.Original_Y` _returnvalue_y)
  (set `self.X_coord` _returnvalue_x)
  (set `self.Y_coord` _returnvalue_y)
  (set `self.Z_coord` _returnvalue_z)
  (for _ (range (* (`self.Length`) (`self.Height`)))
    (bind _returnvalue (`|SpawnActorFromClass` "/Game/DomeKeeper/BP_BlockCube.BP_BlockCube_C" (`KismetMathLibrary.MakeTransform` (`KismetMathLibrary.MakeVector` (`self.X_coord`) (`self.Y_coord`) (`self.Z_coord`))) "AlwaysSpawn" "MultiplyWithRoot" null null))
    (set `/Game/DomeKeeper/BP_BlockCube.HP` (`self.setHP`) _returnvalue)
    (set `self.Y_coord` (+ (`self.Y_coord`) 100.0))
    (bind _result (`/Engine/EditorBlueprintResources/StandardMacros.IncrementInt` (`self.CurrentLenght`))
      (:`  `
        (if (== _result (`self.Length`))
          (set `self.CurrentLenght` 0)
          (set `self.Y_coord` (`self.Original_Y`))
          (set `self.Z_coord` (- (`self.Z_coord`) 100.0))
          (`/Engine/EditorBlueprintResources/StandardMacros.IncrementInt` (`self.setHP`)))))))

(event `Create HUD`
  (bind _returnvalue (`|CreateWidget` "/Game/DomeKeeper/WBP_Score.WBP_Score_C"))
  (`UserWidget.AddToViewport` _returnvalue 0))

(event `IncrementScore`
  (`/Game/DomeKeeper/WBP_Score.Add 100 to Score` (stale `Create HUD` _returnvalue)))

(fn `UserConstructionScript`)