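; BP_BlockCube is a destructible block that randomly holds gold, with a one-in-fifteen chance rolled on BeginPlay; blocks without gold remove their two spheres.
; A first-person projectile hit destroys the projectile and block, incrementing BP_Spawner's score if gold is present.
; Before destruction, DetectionBox jumps through four Y and Z offsets.
; Cube overlaps with another BP_BlockCube destroy this block's CubeFace component.
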(event `self.ReceiveBeginPlay`
  (if (== (`KismetMathLibrary.RandomIntegerInRange` 0 14) 0)
    (set `self.HasGold` true)
    (else
      (`ActorComponent.K2_DestroyComponent` (`self.Sphere`))
      (`ActorComponent.K2_DestroyComponent` (`self.Sphere1`)))))

(event `self.Cube.OnComponentHit`
  (params (HitComponent :type "PrimitiveComponent Object Reference") (OtherActor :type "Actor Object Reference") (OtherComp :type "PrimitiveComponent Object Reference") (NormalImpulse :type "Vector Structure") (Hit :type "HitResult Structure (by ref)"))
  (bind _asbp_first_person_projectile (cast `/Game/FirstPerson/Blueprints/BP_FirstPersonProjectile` OtherActor))
  (`self.K2_DestroyActor` _asbp_first_person_projectile)
  (if (`self.HasGold`)
    (bind _returnvalue (`GameplayStatics.GetActorOfClass` "/Game/DomeKeeper/BP_Spawner.BP_Spawner_C"))
    (`/Game/DomeKeeper/BP_Spawner.IncrementScore` _returnvalue))
  (`SceneComponent.K2_SetRelativeLocation` (`self.DetectionBox`) (0.0 100.0 0.0) false false)
  (`SceneComponent.K2_SetRelativeLocation` (`self.DetectionBox`) (0.0 0.0 100.0) false false)
  (`SceneComponent.K2_SetRelativeLocation` (`self.DetectionBox`) (0.0 -100.0 0.0) false false)
  (`SceneComponent.K2_SetRelativeLocation` (`self.DetectionBox`) (0.0 0.0 -100.0) false false)
  (`self.K2_DestroyActor`))

(event `self.Cube.OnComponentBeginOverlap`
  (params (OverlappedComponent :type "PrimitiveComponent Object Reference") (OtherActor :type "Actor Object Reference") (OtherComp :type "PrimitiveComponent Object Reference") (OtherBodyIndex :type Integer) (bFromSweep :type Boolean) (SweepResult :type "HitResult Structure (by ref)"))
  (bind _cubeface (`self.CubeFace`))
  (cast `/Game/DomeKeeper/BP_BlockCube` OtherActor)
  (`/Engine/EditorBlueprintResources/StandardMacros.IsValid` _cubeface
    (:`Is Valid`
      (`ActorComponent.K2_DestroyComponent` _cubeface))))

(fn `UserConstructionScript`)