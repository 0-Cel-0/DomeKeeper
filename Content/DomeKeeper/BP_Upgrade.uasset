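; BP_Upgrade is a shootable shop actor that sells gun power upgrades for gold.
; On BeginPlay it finds the BP_Spawner, which holds the player's gold and gun power.
; Projectiles hitting its Cube are destroyed and, if gold covers the cost, buy a doubling of gun power.
; Each purchase deducts the cost, raises it by a fixed step, updates the price text and refreshes the spawner's score.
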(event `self.ReceiveBeginPlay`
  (bind _returnvalue (`GameplayStatics.GetActorOfClass` "/Game/DomeKeeper/BP_Spawner.BP_Spawner_C"))
  (set `self.asSpawner` _returnvalue))

(event `self.Cube.OnComponentHit`
  (params (HitComponent :type "PrimitiveComponent Object Reference") (OtherActor :type "Actor Object Reference") (OtherComp :type "PrimitiveComponent Object Reference") (NormalImpulse :type "Vector Structure") (Hit :type "HitResult Structure (by ref)"))
  (bind _asspawner (`self.asSpawner`))
  (bind _cost (`self.Cost`))
  (bind _asspawner_2 (`self.asSpawner`))
  (bind _gold (`/Game/DomeKeeper/BP_Spawner.Gold` _asspawner))
  (bind _asbp_first_person_projectile (cast `/Game/FirstPerson/Blueprints/BP_FirstPersonProjectile` OtherActor))
  (`self.K2_DestroyActor` _asbp_first_person_projectile)
  (if (>= _gold _cost)
    (set `/Game/DomeKeeper/BP_Spawner.Gold` (- _gold _cost) _asspawner)
    (set `/Game/DomeKeeper/BP_Spawner.GunPower` (* (`/Game/DomeKeeper/BP_Spawner.GunPower` _asspawner_2) 2) _asspawner_2)
    (bind _output_get (set `self.Cost` (+ (`self.Cost`) 100)))
    (`TextRenderComponent.K2_SetText` (`self.TextRender`) (`KismetTextLibrary.Conv_IntToText` _output_get))
    (`/Game/DomeKeeper/BP_Spawner.ActualiseScore` _asspawner_2)))

(fn `UserConstructionScript`)